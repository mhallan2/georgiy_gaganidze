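; MyPlayer_BP is the bowling player that aims with the mouse and throws a ball.
; Mouse axes drive controller yaw and inverted pitch.
; A left click spawns a BowlingBall_BP at the camera transform and passes it the camera's forward vector and a fixed launch speed.
; The first player controller then possesses the new ball, so control moves from the player to the ball.
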(event Input|MouseEvents|MouseX
  (params (AxisValue :type Float%20%28single-precision%29))
  ;[1 1 1] Камера
  (Pawn|Input|AddControllerYawInput AxisValue))

(event Input|MouseEvents|MouseY
  (params (AxisValue :type Float%20%28single-precision%29))
  ;[1 1 1] Камера
  (Pawn|Input|AddControllerPitchInput (* AxisValue -1.0)))

(event Input|MouseEvents|LeftMouseButton
  (params (Key :type Key%20Structure :default "None"))
  ;[1 1 1] Бросок и захват контроля
  (:Pressed
    (bind _returnvalue (Game|SpawnActorfromClass "/Game/Bowling/Blueprints/BowlingBall_BP.BowlingBall_BP_C" (Transformation|GetWorldTransform (Variables|Default|GetCamera)) "Undefined" 0 0))
    (Variables|/Game/Bowling/Blueprints/BowlingBall_BP.BowlingBall_BP_C|Setforward _returnvalue (Math|Vector|GetForwardVector (Variables|Default|GetCamera)))
    (Variables|/Game/Bowling/Blueprints/BowlingBall_BP.BowlingBall_BP_C|Setlaunch%20speed _returnvalue 1.5e+03)
    (Pawn|Possess (Game|GetPlayerController 0) _returnvalue)))

(fn ConstructionScript)