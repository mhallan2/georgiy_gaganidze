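; MM_Ball is a rolling physics ball, likely for the main menu, that starts the BizzareBowling level.
; Tick adds axis-driven X velocity to the sphere, capping it both ways, while the spring arm follows and rolls with input.
; Pressing E traces from the camera to a point offset from the sphere and opens the level on any matching object hit.
; BeginPlay plays piano music at the sphere's location.
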(event EventTick
  (params (DeltaSeconds :type Float%20%28single-precision%29))
  (bind _sphere (Variables|Default|GetSphere))
  (bind _returnvalue (Transformation|GetComponentVelocity _sphere))
  (Physics|SetPhysicsLinearVelocity (Variables|Default|GetSphere) (Math|Vector|MakeVector (* (Class|Actor|GetInputAxisKeyValue) -2e+01) 0.0 0.0) true "None")
  (Transformation|SetWorldLocation (Variables|Default|GetSpringArm) (Transformation|GetWorldLocation (Variables|Default|GetSphere)) false false)
  (Transformation|SetWorldRotation (Variables|Default|GetSpringArm) (Math|Rotator|MakeRotator (* (Class|Actor|GetInputAxisKeyValue) -3.0) 0.0 9e+01) false false)
  (if (>= (.x _returnvalue) 4.5e+02)
    (Physics|SetPhysicsLinearVelocity (Variables|Default|GetSphere) (Math|Vector|MakeVector 4.5e+02 0.0 0.0) false "None")
    (elif (<= (.x _returnvalue) -4.5e+02)
      (Physics|SetPhysicsLinearVelocity (Variables|Default|GetSphere) (Math|Vector|MakeVector -4.5e+02 0.0 0.0) false "None"))))

(event EventBeginPlay
  (Audio|PlaySoundatLocation "/Game/Bowling/Audio/Misha_Mozart_-_веселое_пианино__mp3cut_net_.Misha_Mozart_-_веселое_пианино__mp3cut_net_" (Transformation|GetWorldLocation (Variables|Default|GetSphere)) "0, 0, 0" 1.0 1.0 0.0 0 0 0))

(event Input|KeyboardEvents|E
  (params (Key :type Key%20Structure :default "None"))
  (:Pressed
    (bind _returnvalue (Collision|LineTraceForObjects (Transformation|GetWorldLocation (Variables|Default|GetCamera)) (+ (Transformation|GetWorldLocation (Variables|Default|GetSphere)) "0,400.000000,100.000000") (Variables|Default|GetObject%20Types) false 0 "None"))
    (if _returnvalue
      (Game|OpenLevel(byObjectReference) "/Game/Bowling/Levels/BizzareBowling.BizzareBowling"))))

(fn ConstructionScript)