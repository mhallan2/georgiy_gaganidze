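; Bowling lane Blueprint that extends itself along X as the ball travels down it.
; When a BowlingBall_BP enters TriggerZone, it adds a TileHR instance offset by the instance count times DeltaX.
; It then shifts the trigger forward along X for the next overlap and doubles the X scale of Tile.
; SpawnPin is an uncalled stub that only adds a child actor component.
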(event OnComponentBeginOverlap(TriggerZone)
  (params (OverlappedComponent :type Primitive%20Component%20Object%20Reference) (OtherActor :type Actor%20Object%20Reference) (OtherComp :type Primitive%20Component%20Object%20Reference) (OtherBodyIndex :type Integer) (bFromSweep :type Boolean) (SweepResult :type Hit%20Result%20Structure%20%28by%20ref%29))
  (bind _tile (Variables|Default|GetTile))
  (bind _returnvalue (Transformation|GetWorldScale _tile))
  ;[1 1 1] Генерация дорожки
  (Utilities|FlowControl|Sequence
    (:then_0
      (Utilities|Casting|CastToBowlingBall_BP OtherActor)
      (Components|InstancedStaticMesh|AddInstance (Variables|Default|GetTileHR) (Math|Transform|MakeTransform (Math|Vector|MakeVector (* (Components|InstancedStaticMesh|GetInstanceCount (Variables|Default|GetTileHR)) (Variables|Default|Getdelta%20x)) 0.0 0.0) "0, 0, 0" "1,1,1"))
      (Transformation|AddLocalOffset (Variables|Default|GetTriggerZone) "2000.000000,0.000000, 0" false false)
      (Transformation|SetWorldScale3D _tile (Math|Vector|MakeVector (* (.x _returnvalue) 2.0) (.y _returnvalue) (.z _returnvalue))))))

(fn ConstructionScript)

(fn SpawnPin
  (AddComponent|AddChildActorComponent false))