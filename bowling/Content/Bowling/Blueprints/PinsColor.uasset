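; Bowling pin actor that spawns with a random spin and cleans itself up once the ball has passed it.
; On BeginPlay it caches the first BowlingBall_BP in the level and applies a random angular impulse around X to its static mesh.
; Each Tick it compares the mesh's X position to the ball's and destroys itself when it falls more than a set distance behind.
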(event EventTick
  (params (DeltaSeconds :type Float%20%28single-precision%29))
  (Utilities|IsValid (Variables|Default|GetballREF)
    (:Is%20Valid
      (if (< (.x (Transformation|GetWorldLocation (Variables|Default|GetStaticMesh))) (- (.x (Transformation|GetWorldLocation (Variables|/Game/Bowling/Blueprints/BowlingBall_BP.BowlingBall_BP_C|GetmyBall (Variables|Default|GetballREF)))) 1e+03))
        (Actor|DestroyActor)))))

(event EventBeginPlay
  (Utilities|FlowControl|Sequence
    (:then_0
      (bind _outactors (Actor|GetAllActorsOfClass "/Game/Bowling/Blueprints/BowlingBall_BP.BowlingBall_BP_C"))
      (Variables|Default|SetballREF (Utilities|Array|Get(acopy) _outactors)))
    (:then_1
      (Class|PrimitiveComponent|AddAngularImpulseinRadians (Variables|Default|GetStaticMesh) (Math|Vector|MakeVector (Math|Random|RandomFloatinRange -2.0 2.0) 0.0 0.0) "None" true))))

(fn ConstructionScript)