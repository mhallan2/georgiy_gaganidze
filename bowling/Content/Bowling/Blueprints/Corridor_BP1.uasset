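; Bowling corridor Blueprint that extends the lane endlessly in either direction as the ball rolls along it.
; When an MM_Ball overlaps either trigger zone, that side's two instanced mesh components each gain an instance, placed by instance count times a step.
; The trigger then shifts 2000 units further outward, and the shared Tile doubles its X scale.
; SpawnPin only adds a child actor component and is not called here.
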(event OnComponentBeginOverlap(TriggerZone)
  (params (OverlappedComponent :type Primitive%20Component%20Object%20Reference) (OtherActor :type Actor%20Object%20Reference) (OtherComp :type Primitive%20Component%20Object%20Reference) (OtherBodyIndex :type Integer) (bFromSweep :type Boolean) (SweepResult :type Hit%20Result%20Structure%20%28by%20ref%29))
  (bind _tile (Variables|Default|GetTile))
  (bind _returnvalue (Transformation|GetWorldScale _tile))
  ;[1 1 1] Генерация дорожки
  (Utilities|Casting|CastToMM_Ball OtherActor)
  (Components|InstancedStaticMesh|AddInstance (Variables|Default|GetHierRoad) (Math|Transform|MakeTransform (Math|Vector|MakeVector (* (Components|InstancedStaticMesh|GetInstanceCount (Variables|Default|GetHierRoad)) (Variables|Default|Getdelta%20x)) 0.0 0.0) "0, 0, 0" "1,1,1"))
  (Components|InstancedStaticMesh|AddInstance (Variables|Default|GetPlay2) (Math|Transform|MakeTransform (Math|Vector|MakeVector (* (Components|InstancedStaticMesh|GetInstanceCount (Variables|Default|GetPlay2)) (Variables|Default|Getdelta%20x)) 0.0 0.0) "0, 0, 0" "1,1,1"))
  (Transformation|AddLocalOffset (Variables|Default|GetTriggerZone) "2000.000000,0.000000, 0" false false)
  (Transformation|SetWorldScale3D _tile (Math|Vector|MakeVector (* 2 (.x _returnvalue)) (.y _returnvalue) (.z _returnvalue))))

(event OnComponentBeginOverlap(TriggerZone1)
  (params (OverlappedComponent :type Primitive%20Component%20Object%20Reference) (OtherActor :type Actor%20Object%20Reference) (OtherComp :type Primitive%20Component%20Object%20Reference) (OtherBodyIndex :type Integer) (bFromSweep :type Boolean) (SweepResult :type Hit%20Result%20Structure%20%28by%20ref%29))
  (bind _tile (Variables|Default|GetTile))
  (bind _hierroad1 (Variables|Default|GetHierRoad1))
  (bind _play1 (Variables|Default|GetPlay1))
  (bind _returnvalue (Transformation|GetWorldScale _tile))
  ;[1 1 1] Генерация дорожки влево
  (Utilities|Casting|CastToMM_Ball OtherActor)
  (Components|InstancedStaticMesh|AddInstance _hierroad1 (Math|Transform|MakeTransform (Math|Vector|MakeVector (* (Components|InstancedStaticMesh|GetInstanceCount _hierroad1) (Variables|Default|GetNewVar_1)) 0.0 0.0) "0, 0, 0" "1,1,1"))
  (Components|InstancedStaticMesh|AddInstance _play1 (Math|Transform|MakeTransform (Math|Vector|MakeVector (* (Components|InstancedStaticMesh|GetInstanceCount _play1) (Variables|Default|GetNewVar_1)) 0.0 0.0) "0, 0, 0" "1,1,1"))
  (Utilities|FlowControl|Sequence
    (:then_1
      (Transformation|AddLocalOffset (Variables|Default|GetTriggerZone1) "-2000.000000,0.000000, 0" false false)
      (Transformation|SetWorldScale3D _tile (Math|Vector|MakeVector (* 2 (.x _returnvalue)) (.y _returnvalue) (.z _returnvalue))))))

(fn ConstructionScript)

(fn SpawnPin
  (AddComponent|AddChildActorComponent false))