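; Pinspotter is a moving bowling target that brings up the win screen after the ball hits it.
; Tick keeps its collision box on the physics-driven mesh and pushes it along X, faster for a short spell after a ball impact.
; A DoOnce, re-armed outside impacts, counts ball hits.
; When the count is one, a box hit pauses the game after a delay and shows the player's score in the Win widget.
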(event OnComponentHit(Box)
  (params (HitComponent :type Primitive%20Component%20Object%20Reference) (OtherActor :type Actor%20Object%20Reference) (OtherComp :type Primitive%20Component%20Object%20Reference) (NormalImpulse :type Vector :default "0, 0, 0") (Hit :type Hit%20Result%20Structure%20%28by%20ref%29))
  (Utilities|FlowControl|Sequence
    (:then_0
      (Utilities|Casting|CastToBowlingBall_BP OtherActor)
      (Variables|Default|Setimpact true)
      (Utilities|FlowControl|DoOnce false
        (:Completed
          (Math|Integer|IncrementInt (Variables|Default|Getcounter)))))
    (:then_1
      (if (== (Variables|Default|Getcounter) 1)
        (Utilities|FlowControl|Delay 1.0)
        (bind _returnvalue (UserInterface|CreateWidget "/Game/Bowling/Widgets/Win.Win_C"))
        (Variables|Default|SetwinWID _returnvalue)
        (UserInterface|Viewport|AddtoViewport (Variables|Default|GetwinWID) 0)
        (Variables|/Script/Engine.PlayerController|SetbShowMouseCursor (Game|GetPlayerController 0) true)
        (Game|SetGamePaused true)
        (Default|Winscore (Variables|Default|GetwinWID) (Utilities|Text|ToText(Integer) (Variables|/Game/Bowling/Blueprints/MyPlayer_BP.MyPlayer_BP_C|GetscoreMP (Variables|Default|GetplayerREF))))))))

(event EventTick
  (params (DeltaSeconds :type Float%20%28single-precision%29))
  (Utilities|FlowControl|Sequence
    (:then_0
      (Transformation|SetWorldLocation (Variables|Default|GetBox) (Transformation|GetWorldLocation (Variables|Default|GetStaticMesh)) false false))
    (:then_1
      (if (Variables|Default|Getimpact)
        (Physics|SetPhysicsLinearVelocity (Variables|Default|GetStaticMesh) "1000.000000,0.000000,0.000000" false "None")
        (Utilities|FlowControl|Delay 1.6)
        (Variables|Default|Setimpact false)
        (else
          (Utilities|FlowControl|Sequence
            (:then_0
              (Physics|SetPhysicsLinearVelocity (Variables|Default|GetStaticMesh) "300.000000,0.000000,0.000000" false "None"))
            (:then_1
              (Utilities|FlowControl|DoOnce false) ; enters at Reset
            )))))))

(event EventBeginPlay
  (Utilities|FlowControl|Sequence
    (:then_0
      (bind _outactors (Actor|GetAllActorsOfClass "/Game/Bowling/Blueprints/MyPlayer_BP.MyPlayer_BP_C"))
      (Variables|Default|SetplayerREF (Utilities|Array|Get(acopy) _outactors)))
    (:then_1
      (bind _outactors_2 (Actor|GetAllActorsOfClass "/Game/Bowling/Blueprints/BowlingBall_BP.BowlingBall_BP_C"))
      (Variables|Default|Setball%20ref (Utilities|Array|Get(acopy) _outactors_2)))))

(fn ConstructionScript)