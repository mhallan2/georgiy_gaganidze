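; Bowling obstacle actor, built around a pin (Keglya) component, that removes itself once the ball has moved well past it.
; BeginPlay records the pin's world X position and starts a fast looping timer.
; A Box overlap stores the BowlingBall_BP reference, and the timer destroys the actor when that ball's X exceeds the recorded position by a fixed distance.
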(event OnComponentBeginOverlap(Box)
  (params (OverlappedComponent :type Primitive%20Component%20Object%20Reference) (OtherActor :type Actor%20Object%20Reference) (OtherComp :type Primitive%20Component%20Object%20Reference) (OtherBodyIndex :type Integer) (bFromSweep :type Boolean) (SweepResult :type Hit%20Result%20Structure%20%28by%20ref%29))
  (bind _asbowling_ball_bp (Utilities|Casting|CastToBowlingBall_BP OtherActor))
  (Variables|Default|SetAs%20Bowling%20Ball%20BP _asbowling_ball_bp))

(event Custom|CustomEvent_0
  (Utilities|IsValid (Variables|Default|GetAs%20Bowling%20Ball%20BP)
    (:Is%20Valid
      (if (>= (- (Variables|/Game/Bowling/Blueprints/BowlingBall_BP.BowlingBall_BP_C|Getlocation%20x (Variables|Default|GetAs%20Bowling%20Ball%20BP)) (Variables|Default|GetReturn%20Value%20X)) 1e+03)
        (Actor|DestroyActor)))))

(event EventBeginPlay
  (Utilities|FlowControl|Sequence
    (:then_0
      (Variables|Default|SetReturn%20Value%20X (.x (Transformation|GetWorldLocation (Variables|Default|Getkeglya)))))
    (:then_1
      (Utilities|Time|SetTimerbyEvent (delegate Custom|CustomEvent_0) 0.1 true))))

(fn ConstructionScript)