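; Bowling pin spawner that scatters blue and colored pins at random points inside three box volumes, avoiding colliding spawns.
; BeginPlay fills the boxes with hundreds of pins, picking each class by coin flip.
; Once Tick finds a BowlingBall_BP, a DoOnce shifts the boxes forward along X, spawns another batch and sets the ball's BoolForPins.
; Whenever that flag reads false, the DoOnce resets, allowing the next batch further along.
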(event Custom|spawning%20pins
  (bind _returnvalue (Math|Random|RandomBoolwithWeight 0.5))
  (bind _box1 (Variables|Default|GetBox1))
  (bind _box (Variables|Default|GetBox))
  (bind (_origin _boxextent) (Collision|GetComponentBounds _box1))
  (bind (_origin_2 _boxextent_2) (Collision|GetComponentBounds _box))
  (bind _returnvalue_2 (Math|Random|RandomPointinBoundingBox _origin _boxextent))
  (bind _returnvalue_3 (Math|Random|RandomPointinBoundingBox _origin_2 _boxextent_2))
  ;[1 1 1] pin spawn
  (for _index (range 0 200)
    (Utilities|FlowControl|Sequence
      (:then_0
        (if _returnvalue
          (Game|SpawnActorfromClass "/Game/Bowling/Blueprints/PinsBlue.PinsBlue_C" (Math|Transform|MakeTransform _returnvalue_3 "0, 0, 0" "1,1,1") "AdjustIfPossibleButDontSpawnIfColliding" 0 0)
          (else
            (Game|SpawnActorfromClass "/Game/Bowling/Blueprints/PinsColor.PinsColor_C" (Math|Transform|MakeTransform _returnvalue_3 "0, 0, 0" "1,1,1") "AdjustIfPossibleButDontSpawnIfColliding" 0 0))))
      (:then_1
        (if _returnvalue
          (Game|SpawnActorfromClass "/Game/Bowling/Blueprints/PinsBlue.PinsBlue_C" (Math|Transform|MakeTransform _returnvalue_2 "0, 0, 0" "1,1,1") "AdjustIfPossibleButDontSpawnIfColliding" 0 0)
          (else
            (Game|SpawnActorfromClass "/Game/Bowling/Blueprints/PinsColor.PinsColor_C" (Math|Transform|MakeTransform _returnvalue_2 "0, 0, 0" "1,1,1") "AdjustIfPossibleButDontSpawnIfColliding" 0 0)))))))

(event Custom|spawning%20pins%201
  (bind _box2 (Variables|Default|GetBox2))
  (bind (_origin _boxextent) (Collision|GetComponentBounds _box2))
  (bind _returnvalue (Math|Random|RandomPointinBoundingBox _origin _boxextent))
  ;[1 1 1] pin spawn
  (for _index (range 0 100)
    (if (Math|Random|RandomBoolwithWeight 0.5)
      (Game|SpawnActorfromClass "/Game/Bowling/Blueprints/PinsColor.PinsColor_C" (Math|Transform|MakeTransform _returnvalue "0, 0, 0" "1,1,1") "AdjustIfPossibleButDontSpawnIfColliding" 0 0)
      (else
        (Game|SpawnActorfromClass "/Game/Bowling/Blueprints/PinsBlue.PinsBlue_C" (Math|Transform|MakeTransform _returnvalue "0, 0, 0" "1,1,1") "AdjustIfPossibleButDontSpawnIfColliding" 0 0)))))

(event EventTick
  (params (DeltaSeconds :type Float%20%28single-precision%29))
  (bind _box (Variables|Default|GetBox))
  (bind _box2 (Variables|Default|GetBox2))
  (bind _box1 (Variables|Default|GetBox1))
  (bind _returnvalue (Transformation|GetWorldLocation _box2))
  (bind _returnvalue_2 (Transformation|GetWorldLocation _box))
  (bind _returnvalue_3 (Transformation|GetWorldLocation _box1))
  (Utilities|FlowControl|Sequence
    (:then_0
      (bind _outactors (Actor|GetAllActorsOfClass "/Game/Bowling/Blueprints/BowlingBall_BP.BowlingBall_BP_C"))
      (Variables|Default|SetballREF (Utilities|Array|Get(acopy) _outactors))
      (Utilities|IsValid (Variables|Default|GetballREF)
        (:Is%20Valid
          (Utilities|FlowControl|DoOnce false :!label _label
            (:Completed
              (Transformation|SetWorldLocation (Variables|Default|GetBox) (Math|Vector|MakeVector (+ (.x _returnvalue_2) 1.2e+04) (.y _returnvalue_2) (.z _returnvalue_2)) false false)
              (Transformation|SetWorldLocation (Variables|Default|GetBox1) (Math|Vector|MakeVector (+ (.x _returnvalue_3) 1.2e+04) (.y _returnvalue_3) (.z _returnvalue_3)) false false)
              (Transformation|SetWorldLocation (Variables|Default|GetBox2) (Math|Vector|MakeVector (+ (.x _returnvalue) 1.2e+04) (.y _returnvalue) (.z _returnvalue)) false false)
              (CallFunction|SpawningPins)
              (CallFunction|SpawningPins1)
              (Variables|/Game/Bowling/Blueprints/BowlingBall_BP.BowlingBall_BP_C|SetBoolForPins (Variables|Default|GetballREF) true))))))
    (:then_1
      (Utilities|IsValid (Variables|Default|GetballREF)
        (:Is%20Valid
          (if (not (Variables|/Game/Bowling/Blueprints/BowlingBall_BP.BowlingBall_BP_C|GetBoolForPins (Variables|Default|GetballREF)))
            (goto _label Reset)))))))

(event EventBeginPlay
  (CallFunction|SpawningPins)
  (CallFunction|SpawningPins1))

(fn ConstructionScript)