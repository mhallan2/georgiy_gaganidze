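; Spawn area for the bowling game that drops pin obstacles at random points inside its Box bounds.
; A fast looping timer polls the actor's location and, each time it advances over one tile length along X, spawns a regular pin or, rarely, a purple one.
; A separate slower looping timer gives a small random chance of spawning a green pin, independent of movement.
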(event Custom|TickX
  (bind _box (Variables|Default|GetBox))
  (bind _box_2 (Variables|Default|GetBox))
  (bind (_origin _boxextent) (Collision|GetComponentBounds _box))
  (bind (_origin_2 _boxextent_2) (Collision|GetComponentBounds _box_2))
  ;[1 1 1] когда плитка прошла свою длину
  (bind _output_get (Variables|Default|Settick (Transformation|GetActorLocation)))
  (if (> (.x (- _output_get (stale EventBeginPlay _output_get))) 2e+02)
    ;[1 1 1] когда плитка постоянно проходит свою длину
    (bind _output_get_2 (Variables|Default|Setlocation (Variables|Default|Gettick)))
    (if (== (.x (- _output_get _output_get_2)) 0.0)
      ;[1 1 1] спаун обычных кегль
      (if (Math|Random|RandomBoolwithWeight 0.98)
        (Game|SpawnActorfromClass "/Game/Bowling/Blueprints/Obstacle_BP.Obstacle_BP_C" (Math|Conversions|ToTransform(Vector) (Math|Random|RandomPointinBoundingBox _origin _boxextent)) "Undefined" 0 0)
        (else
          ;[1 1 1] спаун фиолетовых кегль
          (Game|SpawnActorfromClass "/Game/Bowling/Blueprints/Obstacle_BP1.Obstacle_BP1_C" (Math|Conversions|ToTransform(Vector) (Math|Random|RandomPointinBoundingBox _origin_2 _boxextent_2)) "Undefined" 0 0))))))

(event Custom|SpawnMarker
  (bind _box (Variables|Default|GetBox))
  (bind (_origin _boxextent) (Collision|GetComponentBounds _box))
  ;[1 1 1] зеленая кегля
  (if (Math|Random|RandomBoolwithWeight 0.02)
    (Game|SpawnActorfromClass "/Game/Bowling/Blueprints/Obstacle_BP2.Obstacle_BP2_C" (Math|Conversions|ToTransform(Vector) (Math|Random|RandomPointinBoundingBox _origin _boxextent)) "Undefined" 0 0)))

(event EventBeginPlay
  (Utilities|FlowControl|Sequence
    (:then_0
      ;[1 1 1] зеленая кегля
      (Utilities|Time|SetTimerbyEvent (delegate Custom|SpawnMarker) 0.5 true))
    (:then_1
      (Utilities|Time|SetTimerbyEvent (delegate Custom|TickX) 0.01 true))
    (:then_2
      ;[1 1 1] когда плитка прошла свою длину
      (Utilities|FlowControl|Delay 0.1)
      (bind _output_get (Variables|Default|Setlocation (Transformation|GetActorLocation))))))

(fn ConstructionScript)